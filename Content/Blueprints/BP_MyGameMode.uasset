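; BP_MyGameMode is a game mode that tracks score and level progress and shows the clear screen.
; On BeginPlay it prints the "number" option from the options string and counts the BP_Light and BP_Flower actors.
; Tick sets Exploding once PassedLights equals the light count.
; AddScore calls GameResult at a score threshold, which adds a selected result widget plus a second, unconditional ClearUI to the viewport.
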(event `self.ReceiveBeginPlay`
  (`KismetSystemLibrary.PrintString` (`GameplayStatics.ParseOption` (`self.OptionsString`) "number"))
  (bind _outactors (`GameplayStatics.GetAllActorsOfClass` "/Game/Blueprints/BP_Light.BP_Light_C"))
  (set `self.NumberOfLights` (`KismetArrayLibrary.Array_Length` _outactors))
  (bind _outactors_2 (`GameplayStatics.GetAllActorsOfClass` "/Game/Blueprints/BP_Flower.BP_Flower_C"))
  (set `self.NumberOfFlowers` (`KismetArrayLibrary.Array_Length` _outactors_2)))

(event `self.ReceiveTick`
  (params (DeltaSeconds :type "Float (single-precision)"))
  (if (== (`self.NumberOfLights`) (`self.PassedLights`))
    (set `self.Exploding` true)))

(event `GameResult`
  (params (Clear :type Boolean))
  (bind _returnvalue (`|CreateWidget` (select `bool` Clear :`true` "/Game/UMG/ClearUI.ClearUI_C" :!type "UserWidget Class Reference")))
  (`UserWidget.AddToViewport` _returnvalue 0)
  (bind _returnvalue_2 (`|CreateWidget` "/Game/UMG/ClearUI.ClearUI_C"))
  (`UserWidget.AddToViewport` _returnvalue_2 0))

(fn `AddScore`
  (bind _output_get (set `self.TotalScore` (+ (`self.TotalScore`) 1)))
  (if (>= _output_get 5)
    (`self.GameResult` true)))

(fn `UserConstructionScript`)